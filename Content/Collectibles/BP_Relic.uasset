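; BP_Relic is a collectible that spins and adds a point to the player's score when collected.
; Tick rotates the mesh by a fixed step each frame, independent of delta time.
; On overlap it disables collision, increments Score on player 0's ThirdPersonCharacter, updates its HUD, plays a coin sound and destroys itself.
; The overlapping actor is never checked, so any overlap credits the player.
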(event `self.ReceiveTick`
  (params (DeltaSeconds :type "Float (single-precision)"))
  ;[1 1 1] Rotates relic and increases player score when collected, then destroys itself.
  (`SceneComponent.K2_AddLocalRotation` (`self.RelicMesh`) (struct :`Yaw` 15.0) false false))

(event `self.CollectCollision.OnComponentBeginOverlap`
  (params (OverlappedComponent :type "PrimitiveComponent Object Reference") (OtherActor :type "Actor Object Reference") (OtherComp :type "PrimitiveComponent Object Reference") (OtherBodyIndex :type Integer) (bFromSweep :type Boolean) (SweepResult :type "HitResult Structure (by ref)"))
  ;[1 1 1] Rotates relic and increases player score when collected, then destroys itself.
  (`PrimitiveComponent.SetCollisionEnabled` (`self.CollectCollision`) "NoCollision")
  (bind _asthird_person_character (cast `/Game/ThirdPersonBP/Blueprints/ThirdPersonCharacter` (`GameplayStatics.GetPlayerCharacter` 0)))
  (bind _output_get (set `/Game/ThirdPersonBP/Blueprints/ThirdPersonCharacter.Score` (+ (`/Game/ThirdPersonBP/Blueprints/ThirdPersonCharacter.Score` _asthird_person_character) 1 0) _asthird_person_character))
  (`/Game/UI/WBP_PlayerHUB.UpdateScore` (`/Game/ThirdPersonBP/Blueprints/ThirdPersonCharacter.PlayerHUDRef` _asthird_person_character) _output_get)
  (`GameplayStatics.PlaySoundAtLocation` "/Game/Audio/coinSound_Cue.coinSound_Cue" (`self.K2_GetActorLocation`) (struct) 1.0 1.0 0.0 null null null)
  (`self.K2_DestroyActor`))

(fn `UserConstructionScript`)