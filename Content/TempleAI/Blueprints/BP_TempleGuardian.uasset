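; Temple guardian AI pawn that chases a seen player and damages them on contact.
; Pawn Sensing writes TargetActor and CanSeePlayer to the controller's Blackboard, and Tick clears them once the target exceeds LosePlayerDistance.
; DamageBox overlap subtracts fixed Health from ThirdPersonCharacter, then sends the HUD that value reduced a second time.
; The trailing Delay has nothing after it, so it does not throttle damage.
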(event `self.ReceiveTick`
  (params (DeltaSeconds :type "Float (single-precision)"))
  ;[1 1 1] Checks distance to player and updates AI Blackboard to chase or stop chasing.
  (bind _asbp_temple_guardian_controller (cast `/Game/TempleAI/AI/BP_TempleGuardianController` (`self.GetController`)))
  (bind _returnvalue (`AIBlueprintHelperLibrary.GetBlackboard` _asbp_temple_guardian_controller))
  (bind _returnvalue_2 (`BlackboardComponent.GetValueAsObject` _returnvalue "TargetActor"))
  (if (!= _returnvalue_2 null)
    (bind _asactor (cast `Actor` _returnvalue_2))
    (if (> (`self.GetDistanceTo` _asactor) (`self.LosePlayerDistance`))
      (`BlackboardComponent.SetValueAsBool` _returnvalue "CanSeePlayer" false)
      (`BlackboardComponent.ClearValue` _returnvalue "TargetActor"))))

(event `self.PawnSensing.OnSeePawn`
  (params (Pawn :type "Pawn Object Reference"))
  ;[1 1 1] Detects player using Pawn Sensing and updates AI Blackboard to start chasing.
  (bind _asbp_temple_guardian_controller (cast `/Game/TempleAI/AI/BP_TempleGuardianController` (`self.GetController`)))
  (bind _blackboard (`AIController.Blackboard` _asbp_temple_guardian_controller))
  (`BlackboardComponent.SetValueAsObject` _blackboard "TargetActor" Pawn)
  (`BlackboardComponent.SetValueAsBool` _blackboard "CanSeePlayer" true))

(event `self.DamageBox.OnComponentBeginOverlap`
  (params (OverlappedComponent :type "PrimitiveComponent Object Reference") (OtherActor :type "Actor Object Reference") (OtherComp :type "PrimitiveComponent Object Reference") (OtherBodyIndex :type Integer) (bFromSweep :type Boolean) (SweepResult :type "HitResult Structure (by ref)"))
  ;[1 1 1] Damages player when close and updates health with delay to prevent rapid damage.
  (bind _asthird_person_character (cast `/Game/ThirdPersonBP/Blueprints/ThirdPersonCharacter` OtherActor))
  (bind _returnvalue (- (`/Game/ThirdPersonBP/Blueprints/ThirdPersonCharacter.Health` _asthird_person_character) 2.0))
  (set `/Game/ThirdPersonBP/Blueprints/ThirdPersonCharacter.Health` _returnvalue _asthird_person_character)
  (`/Game/UI/WBP_PlayerHUB.Update Health` (`/Game/ThirdPersonBP/Blueprints/ThirdPersonCharacter.PlayerHUDRef` _asthird_person_character) _returnvalue (`/Game/ThirdPersonBP/Blueprints/ThirdPersonCharacter.MaxHealth` _asthird_person_character))
  (`KismetSystemLibrary.Delay` 1.0))

(fn `UserConstructionScript`)