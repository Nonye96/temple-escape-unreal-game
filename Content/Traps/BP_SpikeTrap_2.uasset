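; BP_SpikeTrap_2 is a spike trap that damages the third-person character on touching its DamageCollision.
; The overlap plays a hit sound and subtracts fixed damage from Health.
; The HUD update and death check recompute the subtraction from the already reduced Health, so both run one hit ahead.
; Death prints game over, plays a sound and opens TempleLevel_02 after a delay.
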(event `self.DamageCollision.OnComponentBeginOverlap`
  (params (OverlappedComponent :type "PrimitiveComponent Object Reference") (OtherActor :type "Actor Object Reference") (OtherComp :type "PrimitiveComponent Object Reference") (OtherBodyIndex :type Integer) (bFromSweep :type Boolean) (SweepResult :type "HitResult Structure (by ref)"))
  ;[1 1 1] Damage player when touching spike trap
  (bind _asthird_person_character (cast `/Game/ThirdPersonBP/Blueprints/ThirdPersonCharacter` OtherActor))
  (`GameplayStatics.PlaySoundAtLocation` "/Game/Audio/Hit_Cue.Hit_Cue" (`self.K2_GetActorLocation`) (struct) 1.0 1.0 0.0 null null null)
  (bind _returnvalue (- (`/Game/ThirdPersonBP/Blueprints/ThirdPersonCharacter.Health` _asthird_person_character) 20.0))
  (set `/Game/ThirdPersonBP/Blueprints/ThirdPersonCharacter.Health` _returnvalue _asthird_person_character)
  (`/Game/UI/WBP_PlayerHUB.Update Health` (`/Game/ThirdPersonBP/Blueprints/ThirdPersonCharacter.PlayerHUDRef` _asthird_person_character) _returnvalue (`/Game/ThirdPersonBP/Blueprints/ThirdPersonCharacter.MaxHealth` _asthird_person_character))
  (if (<= _returnvalue 0.0)
    (`KismetSystemLibrary.PrintString` "GAME OVER!")
    (`GameplayStatics.PlaySound2D` "/Game/Audio/GameOver_Cue.GameOver_Cue" 1.0 1.0 0.0 null null)
    (`KismetSystemLibrary.Delay` 5.0)
    (`GameplayStatics.OpenLevel` "TempleLevel_02")))

(fn `UserConstructionScript`)